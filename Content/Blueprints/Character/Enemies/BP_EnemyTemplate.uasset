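; Base enemy Blueprint that chases the player's BP_SpriteCharacter and grants it experience when destroyed.
; A detection sphere toggles chasing, and Tick moves the enemy straight toward the player with a swept SetActorLocation scaled by delta time.
; A widget-component health bar refreshes every tick from HealthEnemy.
; UpdateRotation, meant to flip facing by velocity through the AI controller, is unfinished and never called.
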(event `UpdateRotation`
  (bind _returnvalue (`AIBlueprintHelperLibrary.GetAIController` null))
  (bind _returnvalue_2 (`AIBlueprintHelperLibrary.GetAIController` null))
  (bind (_returnvalue_roll _returnvalue_pitch _returnvalue_yaw) (`KismetMathLibrary.BreakRotator` (`Controller.GetControlRotation` _returnvalue)))
  (bind (_returnvalue_roll_2 _returnvalue_pitch_2 _returnvalue_yaw_2) (`KismetMathLibrary.BreakRotator` (`Controller.GetControlRotation` _returnvalue_2)))
  ;[1 1 1] Not Working - supposed to turn enemy actors like my main hero does, but having "controller" issues
  (`/Engine/EditorBlueprintResources/StandardMacros.CompareFloat` (.x (`MovementComponent.Velocity` (`self.CharacterMovement`)))
    (:`>`
      ;;[1 1 1] Look Right
      (`Controller.SetControlRotation` _returnvalue_2 (`KismetMathLibrary.MakeRotator` _returnvalue_roll_2 _returnvalue_pitch_2 (+ _returnvalue_yaw_2 180.0))))
    (:`<`
      ;;[1 1 1] Look Left
      (`Controller.SetControlRotation` _returnvalue (`KismetMathLibrary.MakeRotator` _returnvalue_roll _returnvalue_pitch (+ _returnvalue_yaw -180.0))))))

(event `self.ReceiveBeginPlay`
  (bind _health_enemy (`self.Health_Enemy`))
  ;[1 1 1] On Start, Update UI under health bar (EnemyHealthBarComponent)
  (bind _asenemy_health_ui (cast `/Game/Blueprints/Character/Enemies/EnemyHealthUI/EnemyHealthUI` (`WidgetComponent.GetUserWidgetObject` (`self.EnemyHealthBarWidget`))))
  (set `self.As Enemy Health UI` _asenemy_health_ui)
  (`ProgressBar.SetPercent` (`/Game/Blueprints/Character/Enemies/EnemyHealthUI/EnemyHealthUI.EnemyHealthBar` _asenemy_health_ui) (/ (`/Game/Blueprints/Components/Health_Enemy.CurrentHealth` _health_enemy) (`/Game/Blueprints/Components/Health_Enemy.MaxHealth` _health_enemy)))
  (bind _asbp_sprite_character (cast `/Game/Blueprints/Character/BP_SpriteCharacter` (`GameplayStatics.GetPlayerPawn` 0)))
  (set `self.As BP Sprite Character` _asbp_sprite_character))

(event `self.ReceiveDestroyed`
  ;[1 1 1] When Destroyed, give player xp
  (`/Game/Blueprints/Character/BP_SpriteCharacter.GainExperience` (`self.As BP Sprite Character`) (`self.EnemyExperience`)))

(event `self.ReceiveTick`
  (params (DeltaSeconds :type "Float (single-precision)"))
  (bind _health_enemy (`self.Health_Enemy`))
  (`|ExecutionSequence`
    (:`then_0`
      (if (`self.ChasingPlayer`)
        (`self.K2_SetActorLocation` (+ (`self.K2_GetActorLocation`) (* (`KismetMathLibrary.Normal` (- (`self.K2_GetActorLocation` (`GameplayStatics.GetPlayerPawn` 0)) (`self.K2_GetActorLocation`))) (* (`self.Speed`) DeltaSeconds))) true)))
    (:`then_1`
      ;[1 1 1] Set Health Every Tick
      (`ProgressBar.SetPercent` (`/Game/Blueprints/Character/Enemies/EnemyHealthUI/EnemyHealthUI.EnemyHealthBar` (stale `self.ReceiveBeginPlay` _asenemy_health_ui)) (/ (`/Game/Blueprints/Components/Health_Enemy.CurrentHealth` _health_enemy) (`/Game/Blueprints/Components/Health_Enemy.MaxHealth` _health_enemy))))))

(event `self.EnemyDetectionSphere.OnComponentBeginOverlap`
  (params (OverlappedComponent :type "PrimitiveComponent Object Reference") (OtherActor :type "Actor Object Reference") (OtherComp :type "PrimitiveComponent Object Reference") (OtherBodyIndex :type Integer) (bFromSweep :type Boolean) (SweepResult :type "HitResult Structure (by ref)"))
  ;[1 1 1] Chase "Mechanics"
  (cast `/Game/Blueprints/Character/BP_SpriteCharacter` OtherActor)
  (set `self.ChasingPlayer` true)
  (`KismetSystemLibrary.PrintString` "chasing player"))

(event `self.EnemyDetectionSphere.OnComponentEndOverlap`
  (params (OverlappedComponent :type "PrimitiveComponent Object Reference") (OtherActor :type "Actor Object Reference") (OtherComp :type "PrimitiveComponent Object Reference") (OtherBodyIndex :type Integer))
  ;[1 1 1] Chase "Mechanics"
  (cast `/Game/Blueprints/Character/BP_SpriteCharacter` OtherActor)
  (set `self.ChasingPlayer` false)
  (`KismetSystemLibrary.PrintString` "stop chasing player"))

(fn `UserConstructionScript`)