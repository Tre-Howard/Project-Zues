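; Fire skull enemy Blueprint that deals contact damage and explodes when destroyed.
; AttackBox overlaps damage the other actor's Health component, gated by a DoOnce that resets after a one-second delay.
; On destruction it triggers Explosion, then reuses the overlap event's OtherActor for explosion damage, granting the player experience only if that actor has Health.
; Tick, BeginPlay and construction only call the parent.
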(event `self.ReceiveTick`
  (params (DeltaSeconds :type "Float (single-precision)"))
  (`parent.ReceiveTick` DeltaSeconds))

(event `self.ReceiveBeginPlay`
  (`parent.ReceiveBeginPlay`))

(event `self.AttackBox.OnComponentBeginOverlap`
  (params (OverlappedComponent :type "PrimitiveComponent Object Reference") (OtherActor :type "Actor Object Reference") (OtherComp :type "PrimitiveComponent Object Reference") (OtherBodyIndex :type Integer) (bFromSweep :type Boolean) (SweepResult :type "HitResult Structure (by ref)"))
  (bind _returnvalue (`self.GetComponentByClass` OtherActor "/Game/Blueprints/Components/Health.Health_C"))
  (`/Engine/EditorBlueprintResources/StandardMacros.IsValid` _returnvalue
    (:`Is Valid`
      (`/Engine/EditorBlueprintResources/StandardMacros.DoOnce` false :!label _label
        (:`Completed`
          (`/Game/Blueprints/Components/Health.Take Damage` _returnvalue (`self.Damage`))
          (`KismetSystemLibrary.PrintString` "damage")
          (`KismetSystemLibrary.Delay` 1.0)
          (goto _label :!via `Reset`))))))

(event `self.ReceiveDestroyed`
  (`/Game/Blueprints/Components/Explosion.Explode` (`self.Explosion`))
  (bind _returnvalue (`self.GetComponentByClass` (stale `self.AttackBox.OnComponentBeginOverlap` OtherActor) "/Game/Blueprints/Components/Health.Health_C"))
  (`/Engine/EditorBlueprintResources/StandardMacros.IsValid` _returnvalue
    (:`Is Valid`
      (`/Game/Blueprints/Components/Health.Take Damage` _returnvalue (`self.ExplosionDamage`))
      (`/Game/Blueprints/Character/BP_SpriteCharacter.GainExperience` (`self.As BP Sprite Character`) (`self.EnemyExperience`)))))

(fn `UserConstructionScript`
  (`parent.UserConstructionScript`))