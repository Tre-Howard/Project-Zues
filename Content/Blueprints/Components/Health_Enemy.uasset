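; Enemy health component that tracks current health through damage and healing, destroying its owner at zero.
; BeginPlay creates and caches an EnemyHealthUI widget without displaying it, and caches game instance, game mode and player pawn casts.
; TakeDamage subtracts and prints health, then calls Die, with both gated on a valid BP_FireSkullEnemy reference that is never assigned here.
; Heal adds health and clamps it to MaxHealth.
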(event `self.ReceiveBeginPlay`
  ;[1 1 1] Sets Player UI if actor has Health Component and True
  (if true
    (bind _returnvalue (`|CreateWidget` "/Game/Blueprints/Character/Enemies/EnemyHealthUI/EnemyHealthUI.EnemyHealthUI_C"))
    (set `self.EnemyHealthCache` _returnvalue)
    (`|ExecutionSequence`
      (:`then_0`
        (bind _asproject_zues_game_instance (cast `/Game/Game_ModeInstanceMap/ProjectZues_GameInstance` (`GameplayStatics.GetGameInstance`)))
        (set `self.As Project Zues Game Instance` _asproject_zues_game_instance))
      (:`then_1`
        (bind _asproject_zues_main_game_game_mode (cast `/Game/Game_ModeInstanceMap/ProjectZues_MainGame_GameMode` (`GameplayStatics.GetGameMode`)))
        (set `self.As Project Zues Main Game Game Mode` _asproject_zues_main_game_game_mode))
      (:`then_2`
        (bind _asbp_enemy_template (cast `/Game/Blueprints/Character/Enemies/BP_EnemyTemplate` (`GameplayStatics.GetPlayerPawn` 0)))
        (set `self.As BP Enemy Template` _asbp_enemy_template))
      (:`then_3`
        (bind _asbp_sprite_character (cast `/Game/Blueprints/Character/BP_SpriteCharacter` (`GameplayStatics.GetPlayerPawn` 0)))
        (set `self.As BP Sprite Character` _asbp_sprite_character)))))

(fn `Die`
  ;[1 1 1] Destroy Actor at 0 health
  (`/Engine/EditorBlueprintResources/StandardMacros.IsValid` "/Game/Blueprints/Character/Enemies/BP_FireSkullEnemy.BP_FireSkullEnemy"
    (:`Is Valid`
      (`Actor.K2_DestroyActor` (`self.GetOwner`)))))

(fn `Heal`
  (params (Amount :type "Float (double-precision)"))
  ;[1 1 1] Set Health
  (set `self.CurrentHealth` (+ (`self.CurrentHealth`) Amount))
  ;[1 1 1] Check for Overheal, Don't do it
  (if (>= (`self.CurrentHealth`) (`self.MaxHealth`))
    (set `self.CurrentHealth` (`KismetMathLibrary.FMin` (`self.CurrentHealth`) (`self.MaxHealth`)))))

(fn `Take Damage`
  (params (Amount :type "Float (double-precision)"))
  ;[1 1 1] Take Damage
  (bind _output_get (set `self.CurrentHealth` (- (`self.CurrentHealth`) Amount)))
  (`KismetSystemLibrary.PrintString` (`KismetStringLibrary.Conv_DoubleToString` _output_get))
  (`/Engine/EditorBlueprintResources/StandardMacros.IsValid` "/Game/Blueprints/Character/Enemies/BP_FireSkullEnemy.BP_FireSkullEnemy"
    (:`Is Valid`
      ;[1 1 1] If Health >=0, Die
      ; If health <=1, PlayerFeedback
      (if (<= (`self.CurrentHealth`) 0.0)
        (`/Engine/EditorBlueprintResources/StandardMacros.IsValid` "/Game/Blueprints/Character/Enemies/BP_FireSkullEnemy.BP_FireSkullEnemy"
          (:`Is Valid`
            (`self.Die`)))))))