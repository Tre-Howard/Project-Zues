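; Health component that tracks an actor's current and max health, with damage, healing and death.
; With HasUI set, BeginPlay creates the Player_UI widget and caches game instance, game mode and player sprite character.
; TakeDamage refreshes the health bar and calls Die at zero; Heal clamps to max, refreshing only when reaching it.
; Die calls OnDeath on the cached player character, whichever actor owns the component.
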(event `self.ReceiveBeginPlay`
  ;[1 1 1] Sets Player UI if actor has Health Component and True
  (if (`self.hasUI`)
    (bind _returnvalue (`|CreateWidget` "/Game/Blueprints/UI/Player_UI.Player_UI_C" (`GameplayStatics.GetPlayerController` 0)))
    (bind _output_get (set `self.HealthBarCache` _returnvalue))
    (`UserWidget.AddToViewport` _output_get 0)
    (`Widget.SetVisibility` _output_get "Visible")
    (`|ExecutionSequence`
      (:`then_0`
        (bind _asproject_zues_game_instance (cast `/Game/Game_ModeInstanceMap/ProjectZues_GameInstance` (`GameplayStatics.GetGameInstance`)))
        (set `self.As Project Zues Game Instance` _asproject_zues_game_instance))
      (:`then_1`
        (bind _asproject_zues_main_game_game_mode (cast `/Game/Game_ModeInstanceMap/ProjectZues_MainGame_GameMode` (`GameplayStatics.GetGameMode`)))
        (set `self.As Project Zues Main Game Game Mode` _asproject_zues_main_game_game_mode))
      (:`then_2`
        (bind _asbp_sprite_character (cast `/Game/Blueprints/Character/BP_SpriteCharacter` (`GameplayStatics.GetPlayerPawn` 0)))
        (set `self.As BP Sprite Character` _asbp_sprite_character)))))

(fn `Die`
  (`/Game/Blueprints/Character/BP_SpriteCharacter.OnDeath` (`self.As BP Sprite Character`)))

(fn `Heal`
  (params (Amount :type "Float (double-precision)"))
  ;[1 1 1] Set Health
  (set `self.CurrentHealth` (+ (`self.CurrentHealth`) Amount))
  ;[1 1 1] Check for Overheal, Don't do it
  (if (>= (`self.CurrentHealth`) (`self.MaxHealth`))
    (set `self.CurrentHealth` (`KismetMathLibrary.FMin` (`self.CurrentHealth`) (`self.MaxHealth`)))
    (`self.UpdateUI`)))

(fn `Take Damage`
  (params (Amount :type "Float (double-precision)"))
  ;[1 1 1] Take Damage
  (set `self.CurrentHealth` (- (`self.CurrentHealth`) Amount))
  (`self.UpdateUI`)
  ;[1 1 1] If Health >=0, Die
  ; If health <=1, PlayerFeedback
  (if (<= (`self.CurrentHealth`) 0.0)
    (`self.Die`)))

(fn `UpdateUI`
  (if (`self.hasUI`)
    ;[1 1 1] Gives Progress Bar a Percent To Fill To
    (`/Game/Blueprints/UI/Player_UI.MathForHealthPercent` (`self.HealthBarCache`) (`self.CurrentHealth`) (`self.MaxHealth`))))