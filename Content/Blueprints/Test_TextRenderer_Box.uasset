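; Test box actor that changes the text on a TextRenderTester component when another actor enters or leaves its overlap.
; Begin and end overlap each call SetText on that component through a target reference, each with its own value.
; BeginPlay separately casts the box's owner to Test_TextRender and stores the result.
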(event `self.ReceiveBeginPlay`
  (bind _astest_text_render (cast `/Game/Blueprints/Test_TextRender` (`self.GetOwner`)))
  (set `self.As Test Text Render` _astest_text_render))

(event `self.ReceiveActorBeginOverlap`
  (params (OtherActor :type "Actor Object Reference"))
  (`TextRenderComponent.K2_SetText` (`/Game/Blueprints/Test_TextRender.TextRenderTester` (`self.Target1`)) (`self.Value`)))

(event `self.ReceiveActorEndOverlap`
  (params (OtherActor :type "Actor Object Reference"))
  (`TextRenderComponent.K2_SetText` (`/Game/Blueprints/Test_TextRender.TextRenderTester` (`self.Target1`)) (`self.Value_0`)))

(fn `UserConstructionScript`)